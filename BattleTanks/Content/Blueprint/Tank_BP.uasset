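; Player-controllable tank Blueprint that wires input to movement, aiming and firing components.
; BeginPlay hands the left and right tracks to TankMovement, and the barrel and turret to TankAiming.
; Aim axes add local yaw and pitch to a single scene gimbal, SceneAzimuthGimbo.
; Throttle and turn axes send intents to TankMovement, with both throttles sharing IntendMoveForward, while the fire action calls TankAiming.
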(event `self.ReceiveBeginPlay`
  (`TankMovementComponent.Initialize` (`self.TankMovement`) (`self.LeftTrack`) (`self.RightTrack`))
  (`TankAimingComponent.SetTankComponentPart` (`self.TankAiming`) (`self.TankBarrel`) (`self.TankTurret`)))

(event `InputAxis|AimAzimuth`
  (params (AxisValue :type "Float (single-precision)"))
  ;[1 1 1] Aiming binding
  (`SceneComponent.K2_AddLocalRotation` (`self.Scene_Azimuth_Gimbo`) (`KismetMathLibrary.MakeRotator` 0.0 0.0 AxisValue) false false))

(event `InputAxis|AimElevation`
  (params (AxisValue :type "Float (single-precision)"))
  ;[1 1 1] Aiming binding
  (`SceneComponent.K2_AddLocalRotation` (`self.Scene_Azimuth_Gimbo`) (`KismetMathLibrary.MakeRotator` 0.0 AxisValue) false false))

(event `InputAxis|Forward Throttle`
  (params (AxisValue :type "Float (single-precision)"))
  ;[1 1 1] Movement binding
  (`TankMovementComponent.IntendMoveForward` (`self.TankMovement`) AxisValue))

(event `InputAction|Firing`
  (params (Key :type "Key Structure"))
  ;[1 1 1] firing binding
  (:`Pressed`
    (`TankAimingComponent.Firing` (`self.TankAiming`))))

(event `InputAxis|Backward Throttle`
  (params (AxisValue :type "Float (single-precision)"))
  ;[1 1 1] Movement binding
  (`TankMovementComponent.IntendMoveForward` (`self.TankMovement`) AxisValue))

(event `InputAxis|LeftTurn`
  (params (AxisValue :type "Float (single-precision)"))
  ;[1 1 1] Movement binding
  (`TankMovementComponent.IntendLeftTurn` (`self.TankMovement`) AxisValue))

(event `InputAxis|TurnRight`
  (params (AxisValue :type "Float (single-precision)"))
  ;[1 1 1] Movement binding
  (`TankMovementComponent.IntendRightTurn` (`self.TankMovement`) AxisValue))

(fn `UserConstructionScript`)